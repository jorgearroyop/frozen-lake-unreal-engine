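; FrozenLake toy-text environment that builds a numbered grid board of tiles and holds its reward table.
; On BeginPlay it loads goal, hole and frozen rewards from GI_FL, with start tiles using the frozen reward.
; It parses CustomMap strings into EnvironmentMap, spawns plane meshes and picks each material by tile letter.
; State indices map to row and column, but column uses NumRows, so it assumes a square map.
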(event EventBeginPlay
  ;[0.15 0.15 0.15 0.5] Begin Play
  (Utilities|FlowControl|Sequence
    (:then_0
      (CallFunction|UpdateRewardsfromSettings))
    (:then_1
      (CallFunction|SetupEnvironmentMap)
      (CallFunction|CreateBoardTiles)
      (CallFunction|SetupMaterialsforTiles)
      (CallFunction|CreateTileNumbers) ; TO DO: It's hard coded at the moment
    )))

(fn ConstructionScript)

(fn CreateBoardTiles
  (LocalVariables|SetinitialY (+ (* (- (Variables|Default|GetcenterYaxisInWorld) (/ (Variables|Default|GetnumColumns) 2)) 1e+02) 5e+01))
  (LocalVariables|SetinitialX (- (* (+ (Variables|Default|GetcenterXaxisInWorld) (/ (Variables|Default|GetnumRows) 2)) 1e+02) 5e+01))
  (for _index (range 0 (- (Variables|Default|GetnumRows) 1))
    (for _index_2 (range 0 (- (Variables|Default|GetnumColumns) 1))
      (bind _returnvalue (AddComponent|AddStaticMeshComponent false (Math|Transform|MakeTransform (Math|Vector|MakeVector (- (LocalVariables|GetinitialX) (* _index 100)) (+ (* _index_2 100) (LocalVariables|GetinitialY)) 0.0) "0, 0, 0" "1.000000,1.000000,1.000000")))
      (Components|StaticMesh|SetStaticMesh _returnvalue "/Engine/BasicShapes/Plane.Plane")
      (Utilities|Array|Add (Variables|Default|Gettiles) _returnvalue))))

(fn SetupMaterialsforTiles
  (for (_array_element _array_index) (Variables|Default|Gettiles)
    (bind _value (CallFunction|GetMaterialfromInd _array_index))
    (Rendering|Material|SetMaterial _array_element 0 _value)))

(fn GetMaterialfromInd
  (params (SquareIndex :type Integer))
  (bind _materials (Variables|Default|Getmaterials))
  (bind _environmentmap (Variables|Default|GetenvironmentMap))
  (bind _output (Utilities|Array|Get(acopy) _environmentmap SquareIndex))
  (bind (_value _returnvalue) (Utilities|Map|Find _materials _output))
  (if _returnvalue
    (return _value)
    (else
      (return 0))))

(fn GenerateRandomMap)

(fn SetupEnvironmentMap
  (for _index (range 0 (- (* (Variables|Default|GetnumRows) (Variables|Default|GetnumColumns)) 1))
    (Utilities|Array|Add (Variables|Default|GetenvironmentMap) (Utilities|String|StringToName (Utilities|String|GetSubstring (Utilities|Array|Get(acopy) (Variables|Default|GetcustomMap) (.row (CallFunction|GetRowColfromState _index))) (.col (CallFunction|GetRowColfromState _index)))))))

(fn GetStatefromRowCol
  (params (row :type Integer) (col :type Integer))
  (return (+ (* row (Variables|Default|GetnumColumns)) col)))

(fn GetRowColfromState
  (params (stateInd :type Integer))
  (return (/ stateInd (Variables|Default|GetnumColumns)) (Math|Integer|%(Integer) stateInd (Variables|Default|GetnumRows))))

(fn UpdateRewardsfromSettings
  (Utilities|FlowControl|Sequence
    (:then_0
      (bind _asgi_fl (Utilities|Casting|CastToGI_FL (Game|GetGameInstance)))
      (LocalVariables|SetGIRef _asgi_fl))
    (:then_1
      (Utilities|Map|Add (Variables|Default|Getrewards) "G" (Variables|/Game/Environments/ToyText/FrozenLake/Blueprints/GI_FL.GI_FL_C|GetGoalReward (LocalVariables|GetGIRef)))
      (Utilities|Map|Add (Variables|Default|Getrewards) "H" (Variables|/Game/Environments/ToyText/FrozenLake/Blueprints/GI_FL.GI_FL_C|GetHoleReward (LocalVariables|GetGIRef)))
      (Utilities|Map|Add (Variables|Default|Getrewards) "F" (Variables|/Game/Environments/ToyText/FrozenLake/Blueprints/GI_FL.GI_FL_C|GetFrozenReward (LocalVariables|GetGIRef)))
      (Utilities|Map|Add (Variables|Default|Getrewards) "S" (Variables|/Game/Environments/ToyText/FrozenLake/Blueprints/GI_FL.GI_FL_C|GetFrozenReward (LocalVariables|GetGIRef))))))

(fn CreateTileNumbers
  (for (_array_element _array_index) (Variables|Default|Gettiles)
    (bind _returnvalue (AddComponent|AddTextRenderComponent false (Math|Transform|MakeTransform (+ (Variables|/Script/Engine.SceneComponent|GetRelativeLocation _array_element) "32.000000,32.000000,0.000000") "90.000000,180.000000,0.000000" "1.000000,1.000000,1.000000")))
    (Rendering|Components|TextRender|SetText _returnvalue (Utilities|Text|ToText(Integer) _array_index))))