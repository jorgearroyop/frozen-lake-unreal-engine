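; BP_FuncLib is a utility function library with statistics helpers for float arrays.
; MeanFloatArray sums and averages the array, printing the result, or prints an error and returns zero when it is empty.
; StdDevFloatArray takes the array and a supplied mean, but overwrites rather than accumulates each squared deviation, so only the last element counts.
; It then returns the square root of that value over the length, without an empty-array guard.
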(fn MeanFloatArray
  (params (Array :type Array%20of%20Floats%20%28double-precision%29))
  (bind _returnvalue (Utilities|Array|Length Array))
  (for _array_element Array
    (LocalVariables|SetaSum (+ (LocalVariables|GetaSum) _array_element)))
  (if (> _returnvalue 0)
    (Development|PrintString 0 (Utilities|String|Append "Asum / lenght:   " (Utilities|String|ToString(Float) (/ (LocalVariables|GetaSum) _returnvalue))))
    (return (/ (LocalVariables|GetaSum) _returnvalue))
    (else
      (Development|PrintString 0 "Error: Division by zero!!!" true true "(R=1.000000,G=0.018046,B=0.000000,A=1.000000)" 2e+04)
      (return 0.0))))

(fn StdDevFloatArray
  (params (Array :type Array%20of%20Floats%20%28double-precision%29) (mean :type Float%20%28double-precision%29))
  (for _array_element Array
    (LocalVariables|SetaSum (Math|Float|Square (- _array_element mean))))
  (return (Math|Float|Sqrt (/ (LocalVariables|GetaSum) (Utilities|Array|Length Array)))))